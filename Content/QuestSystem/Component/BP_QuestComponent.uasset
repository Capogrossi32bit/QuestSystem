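; Quest component that tracks a list of runtime quests, their objective progress and their completion.
; AddQuest rejects duplicate IDs and stores new quests as active from their definition.
; It listens to the quest GameState's gameplay objective event, advancing active objectives that match type and target ID, clamped to the required amount.
; Updates write struct copies back into the array, then check completion, with dispatchers announcing start, progress and completion.
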(event Custom|HandleGameplayObjective
  (params (ObjectiveType :type EQuestObjectiveType%20Enum :default "NewEnumerator0") (TargetID :type Name) (Amount :type Integer))
  (for (_array_element _array_index) (Variables|Default|GetActiveQuests)
    (if (and (.isactive _array_element) (not (.iscompleted _array_element)))
      (for (_array_element_2 _array_index_2) (.objectives _array_element)
        (if (and (Utilities|Enum|Equal(Enum) ObjectiveType (.objectivetype _array_element_2)) (== TargetID (.targetid _array_element_2)))
          (CallFunction|UpdateObjectiveProgress _array_index _array_index_2 Amount))))))

(event EventBeginPlay
  (bind _asbp_quest_game_state (Utilities|Casting|CastToBP_QuestGameState (Game|GetGameState)))
  (EventDispatchers|BindEventtoOnGameplayObjectiveEvent _asbp_quest_game_state (delegate Custom|HandleGameplayObjective)))

(fn FindQuestbyID
  (params (QuestID :type Name))
  (bind (_array_element _array_index) (Utilities|Array|ForEachLoopwithBreak (Variables|Default|GetActiveQuests))
    (:LoopBody
      (if (== (.questid _array_element) QuestID)
        (return true (Utilities|Struct|MakeST_QuestRuntime (.questid _array_element) (.questdefinition _array_element) (.objectives _array_element) (.isactive _array_element) (.iscompleted _array_element)) _array_index)))
    (:Completed
      (return false "" 0))))

(fn AddQuest
  (params (QuestDefinition :type PDA%20Quest%20Definition%20Object%20Reference))
  (bind _questid (Variables|/Game/QuestSystem/DataAsset/PDA_QuestDefinition.PDA_QuestDefinition_C|GetQuestID QuestDefinition))
  (bind _objectives (Variables|/Game/QuestSystem/DataAsset/PDA_QuestDefinition.PDA_QuestDefinition_C|GetObjectives QuestDefinition))
  (bind _st_questruntime (Utilities|Struct|MakeST_QuestRuntime _questid QuestDefinition _objectives true))
  (bind _found (CallFunction|FindQuestbyID _questid))
  (if _found
    (Development|PrintString "Ya Existe")
    (else
      (Utilities|Array|Add (Variables|Default|GetActiveQuests) _st_questruntime)
      (Default|CallOnQuestStarted _st_questruntime))))

(fn UpdateObjectiveProgress
  (params (QuestIndex :type Integer) (ObjectiveIndex :type Integer) (Amount :type Integer))
  (bind _activequests (Variables|Default|GetActiveQuests))
  (bind _output (Utilities|Array|Get(acopy) _activequests QuestIndex))
  (bind _output_2 (Utilities|Array|Get(acopy) (.objectives _output) ObjectiveIndex))
  (LocalVariables|SetLocalCopyObjectives (.objectives _output))
  (if (and (> (.requiredamount _output_2) (.currentamount _output_2)) (> Amount 0))
    (bind _structout (Utilities|Struct|SetmembersinST_QuestObjective (Utilities|Array|Get(acopy) (.objectives _output) ObjectiveIndex) (Math|Integer|Min(Integer) (.requiredamount _output_2) (+ (.currentamount _output_2) Amount))))
    (Utilities|Array|SetArrayElem (LocalVariables|GetLocalCopyObjectives) ObjectiveIndex _structout)
    (bind _structout_2 (Utilities|Struct|SetmembersinST_QuestRuntime (Utilities|Array|Get(acopy) (Variables|Default|GetActiveQuests) QuestIndex) (LocalVariables|GetLocalCopyObjectives)))
    (Utilities|Array|SetArrayElem (Variables|Default|GetActiveQuests) QuestIndex _structout_2)
    (Default|CallOnQuestProgressChanged _structout_2)
    (CallFunction|CheckQuestCompleted QuestIndex)))

(fn CheckQuestCompleted
  (params (QuestIndex :type Integer))
  (bind _activequests (Variables|Default|GetActiveQuests))
  (LocalVariables|SetChecker true)
  (for _array_element (.objectives (Utilities|Array|Get(acopy) (Variables|Default|GetActiveQuests) QuestIndex))
    (LocalVariables|SetChecker (and (>= (.currentamount _array_element) (.requiredamount _array_element)) (LocalVariables|GetChecker))))
  (if (LocalVariables|GetChecker)
    (bind _structout (Utilities|Struct|SetmembersinST_QuestRuntime (Utilities|Array|Get(acopy) _activequests QuestIndex) false true))
    (Utilities|Array|SetArrayElem _activequests QuestIndex _structout)
    (Default|CallOnQuestCompleted _structout)
    (else
      (Development|PrintString "no completa"))))